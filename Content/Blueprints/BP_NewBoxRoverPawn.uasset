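; BP_NewBoxRoverPawn is a snake-game pawn that adds sound and visual feedback for eating and dying.
; On BeginPlay it runs the parent's logic, then binds to the OnFoodConsumed and OnSnakeDied dispatchers.
; Food consumption spawns a burst effect at the pawn and plays a ping; death plays an error sound and spawns an explosion.
; The graph holds no movement or scoring logic, and the passed Score is unused.
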(event Custom|OnFoodConsumed_Event
  (params (Score :type Integer))
  (Niagara|SpawnSystematLocation "/Niagara/DefaultAssets/Templates/Systems/RadialBurst.RadialBurst" (Transformation|GetActorLocation))
  (Audio|PlaySound2D "/Engine/EngineSounds/1kSineTonePing.1kSineTonePing" 1.0 1.0 0.0 0 0))

(event Custom|OnSnakeDied_Event
  (Audio|PlaySound2D "/Engine/VREditor/Sounds/UI/Invalid_Action.Invalid_Action" 1.0 1.0 0.0 0 0)
  (Niagara|SpawnSystematLocation "/Niagara/DefaultAssets/Templates/Systems/SimpleExplosion.SimpleExplosion" (Transformation|GetActorLocation)))

(event EventBeginPlay
  (|CallParentFunction)
  (EventDispatchers|BindEventtoOnFoodConsumed (delegate Custom|OnFoodConsumed_Event))
  (EventDispatchers|BindEventtoOnSnakeDied (delegate Custom|OnSnakeDied_Event)))

(event Collision|EventActorBeginOverlap
  (params (OtherActor :type Actor%20Object%20Reference))
  (|CallParentFunction OtherActor) ; 此节点被禁用，将不会被调用。\n从引脚连出引线来编译功能。
)

(event EventTick
  (params (DeltaSeconds :type Float%20%28single-precision%29))
  (|CallParentFunction DeltaSeconds) ; 此节点被禁用，将不会被调用。\n从引脚连出引线来编译功能。
)

(fn ConstructionScript
  (|CallParentFunction))